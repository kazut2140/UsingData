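; BP_DataItemAsset is a placeable item whose mesh and information come from a data asset and which shows its details on screen.
; The construction script, unless RunCode is set, copies the first ItemDataAsset entry matching ItemType into GenericItemInfo and applies its mesh.
; When the player pawn enters SphereCollider, a WBP_WeaponData widget is created once, filled from that info and shown.
; Leaving removes it from the viewport, keeping it for reuse.
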(event OnComponentBeginOverlap(SphereCollider)
  (params (OverlappedComponent :type Primitive%20Component%20Object%20Reference) (OtherActor :type Actor%20Object%20Reference) (OtherComp :type Primitive%20Component%20Object%20Reference) (OtherBodyIndex :type Integer) (bFromSweep :type Boolean) (SweepResult :type Hit%20Result%20Structure%20%28by%20ref%29))
  (if (== OtherActor (Game|Player|GetPlayerPawn 0))
    (Utilities|IsValid (Variables|Default|GetDetailsWidget)
      (:Is%20Valid
        (UserInterface|Viewport|AddtoViewport (Variables|Default|GetDetailsWidget) 0))
      (:Is%20Not%20Valid
        (bind _returnvalue (UserInterface|CreateWidget "/Game/Blueprints/Widget/WBP_WeaponData.WBP_WeaponData_C"))
        (bind _output_get (Variables|Default|SetDetailsWidget _returnvalue))
        (UserInterface|Viewport|AddtoViewport _output_get 0)
        (Default|SetItemDetails (Variables|Default|GetDetailsWidget) (Variables|Default|GetGenericItemInfo))))))

(event OnComponentEndOverlap(SphereCollider)
  (params (OverlappedComponent :type Primitive%20Component%20Object%20Reference) (OtherActor :type Actor%20Object%20Reference) (OtherComp :type Primitive%20Component%20Object%20Reference) (OtherBodyIndex :type Integer))
  (if (== OtherActor (Game|Player|GetPlayerPawn 0))
    (Utilities|IsValid (Variables|Default|GetDetailsWidget)
      (:Is%20Valid
        (Widget|RemovefromParent (Variables|Default|GetDetailsWidget))))))

(event EventBeginPlay)

(event Collision|EventActorBeginOverlap
  (params (OtherActor :type Actor%20Object%20Reference)))

(event EventTick
  (params (DeltaSeconds :type Float%20%28single-precision%29)))

(fn ConstructionScript
  (if (not (Variables|Default|GetbRunCode))
    (bind _array_element (Utilities|Array|ForEachLoopwithBreak (Variables|/Script/UsingData.ItemDataAsset|GetItemInfoArray (Variables|Default|GetItemDataAsset)) :!label _label)
      (:LoopBody
        (if (Utilities|Enum|Equal(Enum) (.ItemType (Utilities|Struct|BreakGenericItemInfo _array_element)) (Variables|Default|GetItemType))
          (Utilities|FlowControl|Sequence
            (:then_0
              (bind _output_get (Variables|Default|SetGenericItemInfo _array_element))
              (Components|StaticMesh|SetStaticMesh (Variables|Character|GetMesh) (Utilities|Struct|BreakGenericItemInfo _output_get)))
            (:then_1
              (goto _label Break))))))))